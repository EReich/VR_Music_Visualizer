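; AudioVisualizer is an actor that plays a music track and shows it as a row of spectrum bars made of spawned cubes.
; On BeginPlay it starts the audio, then SpawnVisual spawns a line of BP_Cube actors centred along Y at fixed world positions.
; Each tick it calculates the track's frequency spectrum at the current game time, one band per cube, and scales each cube's height by that band's magnitude.
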(event `self.ReceiveBeginPlay`
  (`AudioComponent.SetSound` (`self.Audio`) (`self.Track`))
  (`AudioComponent.SetVolumeMultiplier` (`self.Audio`) (`self.Volume`))
  (`AudioComponent.Play` (`self.Audio`) 0.0)
  (`self.SpawnVisual`))

(event `self.ReceiveTick`
  (params (DeltaSeconds :type "Float (single-precision)"))
  (bind _size (`self.Size`))
  (bind _outspectrum (`SoundVisualizationStatics.CalculateFrequencySpectrum` (`self.Track`) 0 (`KismetSystemLibrary.GetGameTimeInSeconds`) 0.1 (`KismetArrayLibrary.Array_Length` (`self.BP_Cube_Array`))))
  (set `self.Spectrum` _outspectrum)
  (for (_array_element _array_index) (`self.BP_Cube_Array`)
    (`self.SetActorScale3D` _array_element (`KismetMathLibrary.MakeVector` _size _size (* (`KismetMathLibrary.Abs` (`|GetArrayItem` (`self.Spectrum`) _array_index)) 0.05)))))

(fn `SpawnVisual`
  (bind _returnvalue (* 100 (`self.Size`)))
  (for _ (range (`self.Number of Cubes`))
    (bind _returnvalue_2 (`|SpawnActorFromClass` "/Game/Blueprints/BP_Cube.BP_Cube_C" (`KismetMathLibrary.MakeTransform` (+ (`KismetMathLibrary.MakeVector` 0.0 (* (`self.Row`) _returnvalue)) (`KismetMathLibrary.MakeVector` 450.0 (/ (* (`self.Number of Cubes`) _returnvalue) -2.0))) (struct)) "AlwaysSpawn" "OverrideRootScale" null null))
    (`KismetArrayLibrary.Array_Add` (`self.BP_Cube_Array`) _returnvalue_2)
    (`/Engine/EditorBlueprintResources/StandardMacros.IncrementInt` (`self.Row`)
      (:`  `
        (if (== (`self.Row`) (`self.Number of Cubes`))
          _)))))

(fn `UserConstructionScript`)